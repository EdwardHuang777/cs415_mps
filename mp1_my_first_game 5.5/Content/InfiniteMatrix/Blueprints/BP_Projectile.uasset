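; BP_Projectile is a projectile actor that destroys enemies it overlaps and awards the player score.
; Each tick it moves along its local X axis by ProjectileSpeed, unscaled by delta time, and it expires after a short delay.
; Hitting a BP_Enemy destroys it, then adds points to the player pawn's Score and shows floating text.
; The projectile destroys itself when an overlap ends with anything other than BP_Player.
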(event EventBeginPlay
  (Utilities|FlowControl|Delay 3.0)
  (Actor|DestroyActor))

(event Collision|EventActorBeginOverlap
  (params (OtherActor :type Actor%20Object%20Reference))
  (bind _asbp_enemy (Utilities|Casting|CastToBP_Enemy OtherActor))
  (Actor|DestroyActor _asbp_enemy)
  (bind _asbp_player (Utilities|Casting|CastToBP_Player (Game|Player|GetPlayerPawn 0)))
  (Variables|/Game/InfiniteMatrix/Blueprints/BP_Player.BP_Player_C|SetScore _asbp_player (+ (Variables|/Game/InfiniteMatrix/Blueprints/BP_Player.BP_Player_C|GetScore _asbp_player) 1e+01))
  (Default|DisplayFloatingText _asbp_player "+10 Score" "(R=1.000000,G=0.979605,B=0.000000,A=1.000000)" "0, 0, 0"))

(event EventTick
  (params (DeltaSeconds :type Float%20%28single-precision%29))
  (Transformation|AddActorLocalOffset (Math|Vector|MakeVector (Variables|Default|GetProjectileSpeed) 0.0 0.0) false false))

(event Collision|EventActorEndOverlap
  (params (OtherActor :type Actor%20Object%20Reference))
  (Utilities|Casting|CastToBP_Player OtherActor
    (:CastFailed
      (Actor|DestroyActor))))

(fn ConstructionScript)